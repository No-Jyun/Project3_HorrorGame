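; BP_LevelTrigger is a box trigger actor that signals BP_ExitGameMode when a level starts.
; Any overlap on the box calls OnLevelStart on the game mode, then disables the box's collision so it does not fire again.
; UpdateCollision re-arms the box with query-only collision, except while the game mode's IsFirstLevelCleared flag is false, when it only sets that flag.
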(event `self.Box.OnComponentBeginOverlap`
  (params (OverlappedComponent :type "PrimitiveComponent Object Reference") (OtherActor :type "Actor Object Reference") (OtherComp :type "PrimitiveComponent Object Reference") (OtherBodyIndex :type Integer) (bFromSweep :type Boolean) (SweepResult :type "HitResult Structure (by ref)"))
  (bind _asbp_exit_game_mode (cast `/Game/Game/BP_ExitGameMode` (`GameplayStatics.GetGameMode`)))
  (`/Game/Game/BP_ExitGameMode.OnLevelStart` _asbp_exit_game_mode)
  (`PrimitiveComponent.SetCollisionEnabled` (`self.Box`) "NoCollision"))

(event `UpdateCollision`
  (bind _asbp_exit_game_mode (cast `/Game/Game/BP_ExitGameMode` (`GameplayStatics.GetGameMode`)))
  (if (`/Game/Game/BP_ExitGameMode.IsFirstLevelCleared` _asbp_exit_game_mode)
    (`PrimitiveComponent.SetCollisionEnabled` (`self.Box`) "QueryOnly")
    (else
      (set `/Game/Game/BP_ExitGameMode.IsFirstLevelCleared` true _asbp_exit_game_mode))))

(fn `UserConstructionScript`)