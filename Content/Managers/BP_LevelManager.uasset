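; Level manager for looping anomaly-judgement levels, choosing where to teleport next among two level indices, each with a reversed variant.
; BeginPlay caches level triggers and sorts teleport points by direction, index and reversal.
; GetNextLevelInfo swaps or flips current/previous level state, returning a spawn point and direction correctness, which is always false going forward.
; UpdateLevel calls UpdateCollision on the previous level's triggers and commits the new level as current.
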(event `self.ReceiveBeginPlay`
  (bind _outactors (`GameplayStatics.GetAllActorsOfClass` "/Game/Actors/BP_LevelTrigger.BP_LevelTrigger_C"))
  (set `self.LevelTriggers` _outactors)
  ;[0.5816 0.1598 0.5644 0.5] 스폰 위치 설정
  (bind _outactors_2 (`GameplayStatics.GetAllActorsOfClass` "/Game/Actors/BP_TeleportPoint.BP_TeleportPoint_C"))
  (for _array_element _outactors_2
    (bind (_isreverse _isbackward _index) (`/Game/Actors/BP_TeleportPoint.GetLevelInformation` _array_element))
    (if _isbackward
      (if _isreverse
        (switch `int` _index
          (:`Default`
            (set `self.BackwardSpawnPoint1_Reverse` _array_element))
          (:`0`
            (set `self.BackwardSpawnPoint0_Reverse` _array_element)))
        (else
          (switch `int` _index
            (:`Default`
              (set `self.BackwardSpawnPoint1` _array_element))
            (:`0`
              (set `self.BackwardSpawnPoint0` _array_element)))))
      (elif _isreverse
        (switch `int` _index
          (:`Default`
            (set `self.ForwardSpawnPoint1_Reverse` _array_element))
          (:`0`
            (set `self.ForwardSpawnPoint0_Reverse` _array_element)))
        (else
          (switch `int` _index
            (:`Default`
              (set `self.ForwardSpawnPoint1` _array_element))
            (:`0`
              (set `self.ForwardSpawnPoint0` _array_element))))))))

(event `UpdateLevel`
  ; 새로운 레벨 시작하면 이전 레벨의 레벨 시작 트리거 다시 키기
  (for _array_element (`self.LevelTriggers`)
    (bind (_isreverse _index) (`/Game/Component/BP_LevelAttributeComponent.GetLevelInformation` (`/Game/Actors/BP_LevelTrigger.LevelAttributeComponent` _array_element)))
    (if (and (== _isreverse (`self.ExIsReverse`)) (== _index (`self.ExLevelIndex`)))
      (`/Game/Actors/BP_LevelTrigger.UpdateCollision` _array_element)))
  (set `self.CurrentLevelIndex` (`self.LevelIndex`))
  (set `self.CurrentIsReverse` (`self.IsReverse`))
  (set `self.IsForwardEntered` false))

(fn `GetNextLevelInfo`
  (params (IsBackward :type Boolean) (IsAnomaly :type Boolean))
  (returns (TeleportPoint :type "Actor Object Reference") (IsRightDirection :type Boolean))
  (locals (TempIndex :type Integer) (TempReverse :type Boolean) (IsCurrentLevel :type Boolean) (IsRightDir :type Boolean))
  (bind _levelindex (`self.LevelIndex`))
  (bind _isreverse (`self.IsReverse`))
  (bind _levelindex_2 (`self.LevelIndex`))
  (bind _levelindex_3 (`self.LevelIndex`))
  (bind _levelindex_4 (`self.LevelIndex`))
  (bind _isrightdir (`local.IsRightDir`))
  (bind _isrightdir_2 (`local.IsRightDir`))
  (bind _isrightdir_3 (`local.IsRightDir`))
  (bind _levelindex_5 (`self.LevelIndex`))
  (bind _returnvalue (and (== (`self.IsReverse`) (`self.CurrentIsReverse`)) (== (`self.LevelIndex`) (`self.CurrentLevelIndex`))))
  (set `local.IsCurrentLevel` _returnvalue)
  (if (== (== IsBackward IsAnomaly) _returnvalue)
    (set `local.IsRightDir` true)
    (else
      (set `local.IsRightDir` false)))
  (if IsBackward
    (if (`local.IsCurrentLevel`)
      ;[0 0.6372 0.06719 0.5] 역방향 - 현재 판정 중인 레벨인 경우
      ; 반대방향 시작지점으로 이동
      (set `self.ExLevelIndex` _levelindex)
      (set `self.LevelIndex` (- 1 _levelindex))
      (set `self.ExIsReverse` _isreverse)
      (set `self.IsReverse` (not _isreverse))
      (if (`self.IsReverse`)
        (switch `int` _levelindex_2
          (:`Default`
            (return (`self.ForwardSpawnPoint1_Reverse`) _isrightdir_3))
          (:`0`
            (return (`self.ForwardSpawnPoint0_Reverse`) _isrightdir_3)))
        (else
          (switch `int` _levelindex_2
            (:`Default`
              (return (`self.ForwardSpawnPoint1`) _isrightdir_3))
            (:`0`
              (return (`self.ForwardSpawnPoint0`) _isrightdir_3)))))
      (else
        ;[0.6198 0.03617 0 0.5] 역방향 - 현재 판정중인 레벨이 아닌 경우 1. 정방향으로 들어간 상태 2. 역방향으로 들어간 상태
        ; 이전 레벨 인덱스 저장 및 Swap
        (set `local.TempIndex` (`self.ExLevelIndex`))
        (set `self.ExLevelIndex` (`self.LevelIndex`))
        (set `self.LevelIndex` (`local.TempIndex`))
        (set `local.TempReverse` (`self.ExIsReverse`))
        (set `self.ExIsReverse` (`self.IsReverse`))
        (set `self.IsReverse` (`local.TempReverse`))
        (if (`self.IsForwardEntered`)
          (set `self.IsForwardEntered` false)
          ;;[0 0.1605 0.6684 0.5] 1번 상태
          (if (`self.IsReverse`)
            (switch `int` _levelindex_3
              (:`Default`
                (return (`self.BackwardSpawnPoint1_Reverse`) _isrightdir_2))
              (:`0`
                (return (`self.BackwardSpawnPoint0_Reverse`) _isrightdir_2)))
            (else
              (switch `int` _levelindex_3
                (:`Default`
                  (return (`self.BackwardSpawnPoint1`) _isrightdir_2))
                (:`0`
                  (return (`self.BackwardSpawnPoint0`) _isrightdir_2)))))
          (else
            ;;[0.6024 0.5548 0 0.5] 2번 상태
            (if (`self.IsReverse`)
              (switch `int` _levelindex_4
                (:`Default`
                  (return (`self.ForwardSpawnPoint1_Reverse`) _isrightdir))
                (:`0`
                  (return (`self.ForwardSpawnPoint0_Reverse`) _isrightdir)))
              (else
                (switch `int` _levelindex_4
                  (:`Default`
                    (return (`self.ForwardSpawnPoint1`) _isrightdir))
                  (:`0`
                    (return (`self.ForwardSpawnPoint0`) _isrightdir)))))))))
    (else
      (set `self.IsForwardEntered` true)
      (set `self.ExLevelIndex` _levelindex_5)
      (bind _output_get (set `self.LevelIndex` (- 1 _levelindex_5)))
      (if (`self.IsReverse`)
        (switch `int` _output_get
          (:`Default`
            (return (`self.ForwardSpawnPoint1_Reverse`) false))
          (:`0`
            (return (`self.ForwardSpawnPoint0_Reverse`) false)))
        (else
          (switch `int` _output_get
            (:`Default`
              (return (`self.ForwardSpawnPoint1`) false))
            (:`0`
              (return (`self.ForwardSpawnPoint0`) false))))))))

(fn `UserConstructionScript`)