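; BP_ExitGameMode is a game mode for an anomaly-spotting level loop where travel direction is judged right or wrong.
; It caches BP_LevelManager and the starting BP_BlockWall on BeginPlay.
; GetNextLevelInfo passes direction and anomaly state to the manager, stores whether the choice was correct and returns a teleport point.
; OnLevelStart prints that result, randomly rolls the next anomaly, updates the level and destroys the start wall.
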(event `self.ReceiveBeginPlay`
  (bind _returnvalue (`GameplayStatics.GetActorOfClass` "/Game/Managers/BP_LevelManager.BP_LevelManager_C"))
  (set `self.LevelManager` _returnvalue)
  (bind _returnvalue_2 (`GameplayStatics.GetActorOfClass` "/Game/Actors/BP_BlockWall.BP_BlockWall_C"))
  (set `self.StartBlock` _returnvalue_2))

(event `OnLevelStart`
  (bind _startblock (`self.StartBlock`))
  (if (`self.IsRightDirection`)
    (`KismetSystemLibrary.PrintString` "Right Direction")
    (else
      (`KismetSystemLibrary.PrintString` "Wrong Direction")))
  (set `self.IsRightDirection` false)
  (bind _output_get (set `self.IsAnomaly` (`KismetMathLibrary.RandomBool`)))
  (if _output_get
    (`KismetSystemLibrary.PrintString` (`KismetStringLibrary.Concat_StrStr` "Current Level Anomaly : " "True"))
    (else
      (`KismetSystemLibrary.PrintString` (`KismetStringLibrary.Concat_StrStr` "Current Level Anomaly : " "false"))))
  (`/Game/Managers/BP_LevelManager.UpdateLevel` (`self.LevelManager`))
  (`/Engine/EditorBlueprintResources/StandardMacros.IsValid` _startblock
    (:`Is Valid`
      (`self.K2_DestroyActor` _startblock))))

(fn `GetNextLevelInfo`
  (params (IsBackward :type Boolean))
  (returns (TeleportPoint :type "Actor Object Reference"))
  (bind (_teleportpoint _isrightdirection) (`/Game/Managers/BP_LevelManager.GetNextLevelInfo` (`self.LevelManager`) IsBackward (`self.IsAnomaly`)))
  (set `self.IsRightDirection` _isrightdirection)
  (return _teleportpoint))

(fn `UserConstructionScript`)